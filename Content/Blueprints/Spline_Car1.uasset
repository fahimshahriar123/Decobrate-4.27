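; Spline car actor that moves a static mesh along its spline when play begins, then destroys itself.
; A timeline track scales the spline length into a distance, and the mesh is placed at that world location with fixed zero rotation and unit scale.
; The timeline update also feeds a delay, so the actor is destroyed about five seconds after movement starts.
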(event `self.ReceiveBeginPlay`
  (bind (_direction _newtrack_0) (`Timeline|Timeline_0`)
    (:`Update`
      (`SceneComponent.K2_SetWorldTransform` (`self.StaticMesh`) (`KismetMathLibrary.MakeTransform` (`SplineComponent.GetLocationAtDistanceAlongSpline` (`self.Spline`) (* (`SplineComponent.GetSplineLength` (`self.Spline`)) _newtrack_0) "World")) false false)
      (`KismetSystemLibrary.Delay` 5.0)
      (`self.K2_DestroyActor`))))

(fn `UserConstructionScript`)