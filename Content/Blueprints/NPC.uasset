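; NPC actor that walks a skeletal mesh along a spline path.
; On BeginPlay it loops the Walking animation and plays a timeline whose track scales the spline length into a distance.
; Each timeline update moves the mesh to that world-space point, without sweep and with fixed zero rotation, so it does not turn to follow the path.
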(event `self.ReceiveBeginPlay`
  (`SkeletalMeshComponent.PlayAnimation` (`self.SkeletalMeshComponent`) "/Game/NPC/Walking.Walking" true)
  (bind (_direction _newtrack_0) (`Timeline|Timeline_0`)
    (:`Update`
      (`SceneComponent.K2_SetWorldTransform` (`self.SkeletalMeshComponent`) (`KismetMathLibrary.MakeTransform` (`SplineComponent.GetLocationAtDistanceAlongSpline` (`self.Spline`) (* (`SplineComponent.GetSplineLength` (`self.Spline`)) _newtrack_0) "World")) false false))))

(fn `UserConstructionScript`)